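; BP_Scotch is a pickup that clears the damaged state of the player character.
; Its Take event acts only if the player is damaged: it resets IsDamaged, hides the Cube and sets Enabled to start a cooldown.
; Tick accumulates time during the cooldown and shows the Cube again after ten seconds.
; Take does not check the cooldown, so it still works while the Cube is hidden.
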(event EventBeginPlay)

(event Collision|EventActorBeginOverlap
  (params (OtherActor :type Actor%20Object%20Reference)))

(event EventTick
  (params (DeltaSeconds :type Float%20%28single-precision%29))
  (if (Variables|Default|GetEnabled)
    (bind _output_get (Variables|Default|SetTimer (+ (Variables|Default|GetTimer) DeltaSeconds)))
    (if (>= _output_get 1e+01)
      (Variables|Default|SetEnabled false)
      (Variables|Default|SetTimer 0.0)
      (Rendering|SetVisibility (Variables|Default|GetCube) true false))))

(event EventTake
  (params (PlayerRef :type BP%20Third%20Person%20Character%20Object%20Reference))
  (Variables|Default|SetAs%20BP%20Third%20Person%20Character PlayerRef)
  (if (Variables|/Game/ThirdPerson/Blueprints/BP_ThirdPersonCharacter.BP_ThirdPersonCharacter_C|GetIsDamaged PlayerRef)
    (Rendering|SetVisibility (Variables|Default|GetCube) false false)
    (Variables|Default|SetEnabled true)
    (Variables|/Game/ThirdPerson/Blueprints/BP_ThirdPersonCharacter.BP_ThirdPersonCharacter_C|SetIsDamaged PlayerRef false)))

(fn ConstructionScript)