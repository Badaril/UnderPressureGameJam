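; BP_Rancher shows the collected parts (parabole, réacteur, hublot) as they are recovered and triggers the game's win screen.
; It caches BP_GameInstance on BeginPlay, and its Take event reads that instance's taken flags to reveal the matching meshes.
; Taking the parabole also reveals the réacteur actor's mesh, and taking the réacteur reveals the hublot's, chaining the objectives.
; Once all three flags are set, Take displays WBP_End_Menu_Win.
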(event EventBeginPlay
  (bind _asbp_game_instance (Utilities|Casting|CastToBP_GameInstance (Game|GetGameInstance)))
  (bind _output_get (Variables|Default|SetAs%20BP%20Game%20Instance _asbp_game_instance)))

(event EventTake
  (params (PlayerRef :type BP%20Third%20Person%20Character%20Object%20Reference))
  (Utilities|FlowControl|Sequence
    (:then_0
      (if (Variables|/Game/Blueprints/Manager/BP_GameInstance.BP_GameInstance_C|GetIsParaboleTaken (stale EventBeginPlay _output_get))
        (Rendering|SetVisibility (Variables|Default|GetSM_parabole_NEW) true false)
        (Rendering|SetVisibility (Variables|/Game/Blueprints/BP_Reacteur.BP_Reacteur_C|GetCube (Variables|Default|GetAs%20BP%20Reacteur)) true false)))
    (:then_1
      (if (Variables|/Game/Blueprints/Manager/BP_GameInstance.BP_GameInstance_C|GetIsReacteurTaken (stale EventBeginPlay _output_get))
        (Rendering|SetVisibility (Variables|Default|GetSM_reacteur_NEW) true false)
        (Rendering|SetVisibility (Variables|/Game/Blueprints/BP_Hublot.BP_Hublot_C|GetHublot (Variables|Default|GetAs%20BP%20Hublot)) true false)))
    (:then_2
      (if (Variables|/Game/Blueprints/Manager/BP_GameInstance.BP_GameInstance_C|GetIsHublotTaken (stale EventBeginPlay _output_get))
        (Rendering|SetVisibility (Variables|Default|GetSM_hublot_NEW) true false)))
    (:then_3
      ;[1 1 1 0.5] win
      (if (Math|Boolean|ANDBoolean (Variables|/Game/Blueprints/Manager/BP_GameInstance.BP_GameInstance_C|GetIsParaboleTaken (stale EventBeginPlay _output_get)) (Variables|/Game/Blueprints/Manager/BP_GameInstance.BP_GameInstance_C|GetIsReacteurTaken (stale EventBeginPlay _output_get)) (Variables|/Game/Blueprints/Manager/BP_GameInstance.BP_GameInstance_C|GetIsHublotTaken (stale EventBeginPlay _output_get)))
        (bind _returnvalue (UserInterface|CreateWidget "/Game/Menu/WBP_End_Menu_Win.WBP_End_Menu_Win_C"))
        (UserInterface|Viewport|AddtoViewport _returnvalue 0)))))

(fn ConstructionScript)