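; BP_Planet is a planet actor whose size and gravity value both derive from its Radius variable.
; The construction script scales the static mesh uniformly by Radius and sets Gravity proportional to the sphere's volume, using a fixed divisor.
; BeginPlay applies the Material variable to the mesh's first slot.
; The file only computes Gravity and does not apply it to other objects.
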(event EventBeginPlay
  (Rendering|Material|SetMaterial (Variables|Default|GetStaticMesh) 0 (Variables|Default|GetMaterial)))

(event Collision|EventActorBeginOverlap
  (params (OtherActor :type Actor%20Object%20Reference)))

(event EventTick
  (params (DeltaSeconds :type Float%20%28single-precision%29)))

(fn ConstructionScript
  (Transformation|SetRelativeScale3D (Variables|Default|GetStaticMesh) (Math|Conversions|ToVector(Float) (/ (Variables|Default|GetRadius) 8e+03)))
  (Variables|Default|SetGravity (/ (* (Math|Float|Power (Variables|Default|GetRadius) 3.0) (Math|Trig|GetPI) (/ 4.0 3.0)) 7e+11)))