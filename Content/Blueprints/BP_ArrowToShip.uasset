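; BP_ArrowToShip is a direction arrow meant to sit on the player character's Head socket, oriented by the BP_Rancher actor's position.
; BeginPlay attempts the attach before the player cast that supplies its parent runs, then finds the rancher and starts a retriggerable-delay loop in place of Tick.
; Each pass sets only yaw, using RInterpTo toward the look-at rotation from rancher to arrow.
; An eased follow-the-player move is left unconnected.
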(event Custom|Repeat
  (CallFunction|ARROWDIR :!label _label)
  (Utilities|FlowControl|RetriggerableDelay 0.01)
  (goto _label))

(event Custom|ARROWDIR
  (Transformation|SetActorRotation (Math|Rotator|MakeRotator 0.0 0.0 (.yaw (Math|Interpolation|RInterpTo (Transformation|GetActorRotation) (Math|Rotator|FindLookatRotation (Transformation|GetWorldLocation (Variables|/Script/Engine.Actor|GetRootComponent (stale EventBeginPlay _returnvalue))) (Transformation|GetActorLocation)) (Utilities|Time|GetWorldDeltaSeconds) 0.0)))))

(event EventTick
  (params (DeltaSeconds :type Float%20%28single-precision%29)))

(event EventBeginPlay
  (Utilities|FlowControl|Sequence
    (:then_0
      (Transformation|AttachActorToActor self (stale _asbp_third_person_character) "Head" "KeepRelative" "KeepRelative" "KeepRelative" true))
    (:then_1
      (bind _returnvalue (Actor|GetActorOfClass "/Game/Blueprints/Rancher/BP_Rancher.BP_Rancher_C"))
      (bind _asbp_third_person_character (Utilities|Casting|CastToBP_ThirdPersonCharacter (Game|GetPlayerCharacter 0)))
      (CallFunction|Repeat))))

(fn ConstructionScript)

(fn Repeater)