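; BP_EnemyAsperge is an asparagus ("Asperge") enemy character that reacts to overlaps with the third-person player.
; When the player overlaps the actor, it caches the player reference and plays a quiet, non-spatial cartoon hit sound.
; A separate Sphere overlap triggers its punch montage, with no damage logic in this graph.
; BeginPlay calls the parent and sets an Alpha value that this graph never reads.
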(event OnComponentBeginOverlap(Sphere)
  (params (OverlappedComponent :type Primitive%20Component%20Object%20Reference) (OtherActor :type Actor%20Object%20Reference) (OtherComp :type Primitive%20Component%20Object%20Reference) (OtherBodyIndex :type Integer) (bFromSweep :type Boolean) (SweepResult :type Hit%20Result%20Structure%20%28by%20ref%29))
  (Utilities|Casting|CastToBP_ThirdPersonCharacter OtherActor)
  (Animation|PlayAnimMontage "/Game/Enemies/Mesh/Asperge/asperge_punch_Montage.asperge_punch_Montage" 1.0 "None"))

(event EventBeginPlay
  (|CallParentFunction)
  (Variables|Default|SetAlpha 0.06))

(event Collision|EventActorBeginOverlap
  (params (OtherActor :type Actor%20Object%20Reference))
  (bind _asbp_third_person_character (Utilities|Casting|CastToBP_ThirdPersonCharacter OtherActor))
  (Variables|Default|SetAs%20BP%20Third%20Person%20Character_0 _asbp_third_person_character)
  (Audio|PlaySound2D "/Game/sounds/universfield-cartoon-wet-hit-352447.universfield-cartoon-wet-hit-352447" 0.1 1.0 0.0 0 0))

(event EventTick
  (params (DeltaSeconds :type Float%20%28single-precision%29))
  (|CallParentFunction DeltaSeconds) ; This node is disabled and will not be called.\nDrag off pins to build functionality.
)

(fn ConstructionScript
  (|CallParentFunction))