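; Parent enemy Character that chases the player, with planet-centred gravity support.
; BeginPlay checks for an overlapped BP_Planet to copy its centre and gravity scale, and a looping timer re-aims gravity toward that centre.
; Tick eases location toward the player and copies their rotation.
; Sphere overlap launches the player and flags damage or drains O2 if already damaged, while Death teleports the enemy to its respawn location.
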(event OnComponentBeginOverlap(Sphere)
  (params (OverlappedComponent :type Primitive%20Component%20Object%20Reference) (OtherActor :type Actor%20Object%20Reference) (OtherComp :type Primitive%20Component%20Object%20Reference) (OtherBodyIndex :type Integer) (bFromSweep :type Boolean) (SweepResult :type Hit%20Result%20Structure%20%28by%20ref%29))
  (bind _asbp_third_person_character (Utilities|Casting|CastToBP_ThirdPersonCharacter OtherActor))
  (Character|LaunchCharacter _asbp_third_person_character (* (Math|Vector|GetForwardVector (Variables|Default|GetPushDirection)) 1.5e+03) false false)
  (if (Variables|/Game/ThirdPerson/Blueprints/BP_ThirdPersonCharacter.BP_ThirdPersonCharacter_C|GetIsDamaged _asbp_third_person_character)
    (Variables|/Game/ThirdPerson/Blueprints/BP_ThirdPersonCharacter.BP_ThirdPersonCharacter_C|SetO2Level _asbp_third_person_character (Math|Float|Clamp(Float) (- (Variables|/Game/ThirdPerson/Blueprints/BP_ThirdPersonCharacter.BP_ThirdPersonCharacter_C|GetO2Level _asbp_third_person_character) 0.01)))
    (else
      (Variables|/Game/ThirdPerson/Blueprints/BP_ThirdPersonCharacter.BP_ThirdPersonCharacter_C|SetIsDamaged _asbp_third_person_character true)
      (Variables|/Game/ThirdPerson/Blueprints/BP_ThirdPersonCharacter.BP_ThirdPersonCharacter_C|SetScotchCooldown _asbp_third_person_character 0.0))))

(event Custom|InitGravityTimer
  (Utilities|Time|SetTimerbyEvent (delegate Custom|Gravity) 0.05 true false -0.05))

(event Custom|Gravity
  (Utilities|FlowControl|Sequence
    (:then_0
      (if (Variables|Default|GetPlanetSide?)
        (Class|CharacterMovementComponent|SetGravityDirection (Variables|Character|GetCharacterMovement) (Math|Vector|GetUnitDirection(Vector) (Transformation|GetActorLocation) (Variables|Default|GetPlanetCenterLoc)))))))

(event Custom|Death
  (Transformation|SetActorLocation (Variables|Default|GetRespawnLocation) false false))

(event EventTick
  (params (DeltaSeconds :type Float%20%28single-precision%29))
  ;[0.15 0.15 0.15 0.5] Chase Player
  (Transformation|SetActorLocation (Math|Interpolation|Ease "Linear" 0.02 (Transformation|GetActorLocation) (Transformation|GetActorLocation (Game|Player|GetPlayerPawn 0))) false false)
  (Transformation|SetActorRotation (Transformation|GetActorRotation (Game|Player|GetPlayerPawn 0))))

(event EventBeginPlay
  (Utilities|FlowControl|Sequence
    (:then_0
      (CallFunction|InitGravityTimer))
    (:then_1
      (if (Collision|IsOverlappingActor (Utilities|Array|Get(acopy) (Collision|GetOverlappingActors "/Game/Blueprints/BP_Planet.BP_Planet_C" :!class /Script/Engine.Actor)) :!class /Script/Engine.Actor)
        (CallFunction|SideON)
        (else
          (CallFunction|SideOFF))))))

(fn ConstructionScript)

(fn SideOFF)

(fn SideON
  (bind _overlappingactors (Collision|GetOverlappingActors "/Game/Blueprints/BP_Planet.BP_Planet_C" :!class /Script/Engine.Actor))
  (bind _output (Utilities|Array|Get(acopy) _overlappingactors))
  (Variables|Default|SetPlanetSide? true)
  (Variables|Default|SetPlanetCenterLoc (Transformation|GetActorLocation _output))
  (Variables|/Script/Engine.CharacterMovementComponent|SetGravityScale (Variables|Character|GetCharacterMovement) (Variables|/Game/Blueprints/BP_Planet.BP_Planet_C|GetGravity _output))
  (Physics|SetEnableGravity (Variables|Collision|GetCapsuleComponent) true)
  (Pawn|Components|CharacterMovement|SetMovementMode (Variables|Character|GetCharacterMovement) "MOVE_Falling" 0)
  (CallFunction|InitGravityTimer))

(fn MoveTowardsPlayer)

(fn InitGravityTimer)

(fn SetPlanetside)

(fn SetOffPlanet)