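; Enemy character that knocks the third-person player away on contact and has logic to chase them.
; BeginPlay sets walk speed and calls MoveTowardsPlayer, which is empty.
; ChasePlayer runs AI MoveTo on the player, then calls that empty function; nothing here triggers ChasePlayer.
; Sphere overlap launches the player along PushDirection, then after a short delay switches their capsule to physics simulation with physics-only collision.
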(event OnComponentBeginOverlap(Sphere)
  (params (OverlappedComponent :type Primitive%20Component%20Object%20Reference) (OtherActor :type Actor%20Object%20Reference) (OtherComp :type Primitive%20Component%20Object%20Reference) (OtherBodyIndex :type Integer) (bFromSweep :type Boolean) (SweepResult :type Hit%20Result%20Structure%20%28by%20ref%29))
  (bind _asbp_third_person_character (Utilities|Casting|CastToBP_ThirdPersonCharacter OtherActor))
  (Character|LaunchCharacter _asbp_third_person_character (* (Math|Vector|GetForwardVector (Variables|Default|GetPushDirection)) 2e+03) false false)
  (Utilities|FlowControl|Delay 0.2)
  (Physics|SetSimulatePhysics (Variables|/Script/Engine.Character|GetCapsuleComponent _asbp_third_person_character) true)
  (Collision|SetCollisionEnabled (Variables|/Script/Engine.Character|GetCapsuleComponent _asbp_third_person_character) "PhysicsOnly"))

(event Custom|ChasePlayer
  (bind _asbp_third_person_character (Utilities|Casting|CastToBP_ThirdPersonCharacter (Game|GetPlayerCharacter 0)))
  (bind _output_get (Variables|Default|SetPlayerRef _asbp_third_person_character))
  (AI|AIMoveTo self "0, 0, 0" _output_get 5.0 false
    (:OnSuccess
      _)
    (:OnFail
      _))
  (CallFunction|MoveTowardsPlayer))

(event EventBeginPlay
  (Variables|/Script/Engine.CharacterMovementComponent|SetMaxWalkSpeed (Variables|Character|GetCharacterMovement) 4e+02)
  (CallFunction|MoveTowardsPlayer))

(fn ConstructionScript)

(fn MoveTowardsPlayer)