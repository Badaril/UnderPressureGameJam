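; BP_Enemy2 is an enemy that chases the player and knocks them away on contact.
; On BeginPlay it lowers its walk speed and starts an AI MoveTo toward the third-person character, reissuing the move whenever it succeeds or fails.
; Overlapping its Sphere launches that character along the PushDirection component's up vector, so that component's rotation sets the push direction.
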(event OnComponentBeginOverlap(Sphere)
  (params (OverlappedComponent :type Primitive%20Component%20Object%20Reference) (OtherActor :type Actor%20Object%20Reference) (OtherComp :type Primitive%20Component%20Object%20Reference) (OtherBodyIndex :type Integer) (bFromSweep :type Boolean) (SweepResult :type Hit%20Result%20Structure%20%28by%20ref%29))
  (bind _asbp_third_person_character (Utilities|Casting|CastToBP_ThirdPersonCharacter OtherActor))
  (Character|LaunchCharacter _asbp_third_person_character (* (Math|Vector|GetUpVector (Variables|Default|GetPushDirection)) 1e+03) false false))

(event Custom|MoveTowardsPlayer
  (bind _asbp_third_person_character (Utilities|Casting|CastToBP_ThirdPersonCharacter (Game|GetPlayerCharacter 0)))
  (bind _output_get (Variables|Default|SetPlayerRef _asbp_third_person_character))
  (AI|AIMoveTo self "0, 0, 0" _output_get 5.0 false
    (:OnSuccess
      _)
    (:OnFail
      _))
  (CallFunction|MoveTowardsPlayer))

(event EventBeginPlay
  (Variables|/Script/Engine.CharacterMovementComponent|SetMaxWalkSpeed (Variables|Character|GetCharacterMovement) 2e+02)
  (CallFunction|MoveTowardsPlayer))

(fn ConstructionScript)