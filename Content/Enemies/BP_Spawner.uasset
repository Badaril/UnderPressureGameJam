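; Enemy spawner actor that spawns a limited number of enemies at its spawn point, one at a time.
; BeginPlay spawns the first unconditionally, setting each enemy's respawn location to that point and starting a cooldown.
; Tick accumulates delta time through a fixed two-second cooldown, prints it, then decrements the remaining count and spawns again while it stays positive.
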(event Custom|spawnMonster
  (bind _spawnpoint (Variables|Default|GetSpawnPoint))
  (bind _returnvalue (Game|SpawnActorfromClass (Variables|Default|GetEnnemy) (Transformation|GetWorldTransform _spawnpoint) "Undefined" "MultiplyWithRoot" 0 0))
  (Variables|/Game/Enemies/BP_EnemyParent.BP_EnemyParent_C|SetRespawnLocation _returnvalue (Transformation|GetWorldLocation _spawnpoint))
  (Variables|Default|SetInCooldown true))

(event EventBeginPlay
  (CallFunction|SpawnMonster))

(event Collision|EventActorBeginOverlap
  (params (OtherActor :type Actor%20Object%20Reference)))

(event EventTick
  (params (DeltaSeconds :type Float%20%28single-precision%29))
  (if (Variables|Default|GetInCooldown)
    (bind _output_get (Variables|Default|SetCooldown (+ (Variables|Default|GetCooldown) DeltaSeconds)))
    (if (>= _output_get 2.0)
      (Development|PrintString (Utilities|String|ToString(Float) _output_get))
      (Variables|Default|SetInCooldown false)
      (Variables|Default|SetNumber (- (Variables|Default|GetNumber) 1))
      (Variables|Default|SetCooldown 0.0))
    (elif (> (Variables|Default|GetNumber) 0)
      (CallFunction|SpawnMonster))))

(fn ConstructionScript)