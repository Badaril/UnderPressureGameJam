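; A decor billboard tree that turns about its vertical axis to follow the player's camera.
; BeginPlay applies its Material to the Plane, caches the third-person character and starts a 0.01-second retriggerable-delay loop instead of using Tick.
; Each pass sets only the actor's yaw from the look-at rotation from FollowCamera to the tree, passed through RInterpTo with no interp speed set.
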(event Custom|DecorRotation
  (Transformation|SetActorRotation (Math|Rotator|MakeRotator 0.0 0.0 (.yaw (Math|Interpolation|RInterpTo (Transformation|GetActorRotation) (Math|Rotator|FindLookatRotation (Transformation|GetWorldLocation (Variables|/Game/ThirdPerson/Blueprints/BP_ThirdPersonCharacter.BP_ThirdPersonCharacter_C|GetFollowCamera (stale EventBeginPlay _asbp_third_person_character))) (Transformation|GetActorLocation)) (Utilities|Time|GetWorldDeltaSeconds) 0.0)))))

(event Custom|Repeater
  (CallFunction|DecorRotation :!label _label)
  (Utilities|FlowControl|RetriggerableDelay 0.01)
  (goto _label))

(event EventBeginPlay
  (Utilities|FlowControl|Sequence
    (:then_0
      (Rendering|Material|SetMaterial (Variables|Default|GetPlane) 0 (Variables|Default|GetMaterial)))
    (:then_1
      (bind _asbp_third_person_character (Utilities|Casting|CastToBP_ThirdPersonCharacter (Game|GetPlayerCharacter 0)))
      (CallFunction|Repeater))))

(fn ConstructionScript)